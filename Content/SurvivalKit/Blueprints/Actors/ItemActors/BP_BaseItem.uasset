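; Base item actor for the Survival Kit, providing the shared drop, quick-use and use-sound behavior for items.
; BeginPlay caches the SurvivalKitComponent from the controller reference.
; Dropping has that component drop the item's slot on the server, then destroys the actor through a multicast event.
; QuickUseItem is a placeholder that prints a not-implemented warning, and a client event plays the 2D use sound from the item information.
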(event Custom|DestroyItemMulticast
  ;[0 0.9802 1] Destroy Item
  (Actor|DestroyActor))

(event Custom|PlayItemUsedSoundClient
  ;[0 0.1374 1] Play Item Used Sound
  (GeneralFunctions|PlayItemUsedSound))

(event EventBeginPlay
  ;[1 0.01713 0] Event BeginPlay
  (bind _controllerreference (Variables|NonEditablePart|GetControllerReference)
    (:then
      (bind _returnvalue (CallFunction|GetSurvivalKitComponent _controllerreference))
      (Variables|Default|SetSurvivalKitComponent _returnvalue))
    (:else)))

(event EventActionDropItem
  ;[0.2281 1 0] Drop Item Interface Function
  (GeneralFunctions|DropItem))

(fn ConstructionScript)

(fn QuickUseItem
  (Development|PrintString "Quick Use Item Function Not Implemented For This Item.(If You Don't Know How To Implement Use Function, Please Read The Documentation.)" true true "(R=0.000000,G=0.660000,B=1.000000,A=1.000000)" 7.5))

(fn GetItemInformation
  (return 0))

(fn DropItem
  (Default|DropSlotItemServer (Variables|Default|GetSurvivalKitComponent) (Variables|InventorySystem|GetSlotID))
  (CallFunction|DestroyItemMulticast))

(fn PlayItemUsedSound
  (bind _siteminformation (Variables|NonEditablePart|GetSItemInformation))
  (bind _sitemwidgetsoundsettings (Utilities|Struct|BreakS_ItemInformation _siteminformation))
  (bind _itemonused (Utilities|Struct|BreakS_ItemWidgetSoundSettings _sitemwidgetsoundsettings))
  (if (Utilities|Array|IsEmpty (Utilities|GetDisplayName _itemonused))
    (Development|PrintString "Sound Empty" true true "(R=1.000000,G=0.036552,B=0.000000,A=1.000000)"))
  (Audio|PlaySound2D _itemonused 1.0 1.0 0.0 0 0))