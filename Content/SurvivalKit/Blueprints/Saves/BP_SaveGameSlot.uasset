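; Save game object for the survival kit that holds a player's inventory information, favourited craft items and basic attribute values.
; Events write the data: inventory info is replaced whole, favourites are added or removed, and attribute values are stored in a map keyed by attribute class.
; Getters return each piece, with attribute lookups also reporting whether the class is registered.
; A flag records whether the inventory has been initialized.
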(event EventSetSaveGameInformations
  (params (SaveGameInformation :type S%20Save%20Game%20Inventory%20Info%20Structure))
  ;[1 0.532 0] Set Game Information
  (Variables|SaveSystem|SetSSaveGameInventoryInfo SaveGameInformation))

(event EventSetBasicAttributeValue
  (params (BasicAttrbiuteClass :type BP%20Basic%20Attribute%20Component%20Class%20Reference) (ValueToSet :type Float%20%28double-precision%29))
  ;[1 0.532 0] Set Game Information
  (Utilities|Map|Add (Variables|SaveSystem|GetBasicAttributes) BasicAttrbiuteClass ValueToSet))

(event EventAddSaveGameFavItem
  (params (FavouritedItem :type E_Item%20Enum :default "NewEnumerator1"))
  ;[1 0.532 0] Set Game Information
  (Utilities|Array|Add (Variables|SaveSystem|GetFavouritedCraftItems) FavouritedItem))

(event EventRemoveSaveGameFavItem
  (params (EItem :type E_Item%20Enum :default "NewEnumerator1"))
  ;[1 0.532 0] Set Game Information
  (Utilities|Array|RemoveItem (Variables|SaveSystem|GetFavouritedCraftItems) EItem))

(event EventSetIsInventoryInitialized
  (params (IsInventoryInitialized :type Boolean))
  ;[1 0.532 0] Set Game Information
  (Variables|SaveSystem|SetIsInventoryInitialized IsInventoryInitialized))

(fn GetBasicAttributeValue
  (params (TargetClass :type BP%20Basic%20Attribute%20Component%20Class%20Reference))
  (bind _basicattributes (Variables|SaveSystem|GetBasicAttributes))
  (bind (_value _returnvalue) (Utilities|Map|Find _basicattributes TargetClass))
  (return _value _returnvalue))

(fn GetIsInventoryInitialized
  (return (Variables|SaveSystem|GetIsInventoryInitialized)))

(fn GetSaveGameFavItems
  (return (Variables|SaveSystem|GetFavouritedCraftItems)))

(fn GetSaveGameInformations
  (return (Variables|SaveSystem|GetSSaveGameInventoryInfo)))