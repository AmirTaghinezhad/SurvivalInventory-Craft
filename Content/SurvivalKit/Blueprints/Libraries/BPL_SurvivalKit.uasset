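; BPL_SurvivalKit is a Blueprint function library of shared lookup helpers for the survival kit.
; It fetches the survival kit component from a controller's pawn through the BPI_General interface.
; Item and crafting data come from DT_ItemList and DT_CraftingList, using the item enum's string as row name, with a fallback struct for missing items.
; A linear search finds skin details by name and reports success.
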(fn GetSurvivalKitComponent
  (params (ControllerReference :type Controller%20Object%20Reference))
  (bind _returnvalue (Pawn|GetControlledPawn ControllerReference))
  (if (Utilities|DoesObjectImplementInterface _returnvalue "/Game/SurvivalKit/Blueprints/Interfaces/BPI_General.BPI_General_C")
    (bind _returnvalue_2 (Class|BPIGeneral|GetSurvivalKitComponent(Message) _returnvalue))
    (return _returnvalue_2)))

(fn GetItemInformationbyEnum
  (params (EItem :type E_Item%20Enum :default "NewEnumerator1"))
  (bind _returnvalue (Utilities|GetDataTableRow "/Game/SurvivalKit/Blueprints/Datatables/DT_ItemList.DT_ItemList" (Utilities|String|StringToName (Utilities|String|EnumtoString EItem)))
    (:then
      (return _returnvalue))
    (:RowNotFound
      (return (Utilities|Struct|MakeS_ItemInformation "NewEnumerator1" "" 1 0 "(ItemName_19_024C8A504C8AB45854AE8BABD09CD1AC=\"\",ItemImage_2_3AC975A54587B86B1D096DABFBEAEF88=None,ItemMesh_6_E942D591476215773F1DBCB149CBD72A=None)" "(ItemOnClickedSound_23_D85EB52443CF6EBCD9B8D6AF1DF5CA5D=None,ItemOnReleasedSound_24_BB5FCF3D4C9021B4EF44E68E7CDC5723=None,ItemOnUsed_25_93F0EC90468C0AE1A5764C875A6EC7F6=None,OnDrop_28_88C2E7B64B7F813AFD71CDA013F62ACE=None)" "(SItemLocalOffset_9_DD9AF2514CE0C73296D68FA572FC8167=(X=0.000000,Y=0.000000,Z=0.000000),SItemRotation_7_EDB032FB414FC31DF703DD918EC1BC7D=(Pitch=0.000000,Yaw=0.000000,Roll=0.000000),SItemScale_8_76AED81541DA9460F2911E98A6A325BD=(X=1.000000,Y=1.000000,Z=1.000000))" "(IsSimulatingPhysics_1_924DEB144008C79E51800B8CFC3F560A=True,SMassInKgSettings_36_134A6728493565877D25C28447BE8F66=(BoneName_7_1495074040896FCDF1CF6AA1080E75AE=\"\",IsMassInKgEnabled_1_60C08ABE43C2361315CDC89CE1D5F1AD=False,MassInKg_4_92CCA68D4381AF7F0FBA0AA86EC6217A=0.000000),LinearDamping_11_6C55414E4FADD00395914EB97FD8CAF7=0.010000,AngularDamping_13_D7C7ED4B4B9312F3880AB49460F2592A=0.000000,EnableGravity_16_42C8CBE540C19A33481EC58B037A9AE6=True,IgnoreRadialImpulse_18_4D656DC54E50815000367BA627797441=False,IngoreRadialForce_21_11060A3A45DD808F375C6A96D7DDB706=False,ApplyImpulseOnDamage_32_F15A6F8E42E94ADBB4AF6CAF0959B72B=True,ReplicatePhyiscsToAutonomousProxy_30_941D82574A8BACC41275EAB5AFF389F7=True)" "(ImpulseMultiplier_24_1A9B26894C3A077C657AD7B3C427A9F1=0.000000,BoneName_20_8160FDE34E156963A81550B3F09D2AE7=\"\",VelChange_21_C96088BB427C13BBB753F8B78AEC6F0A=True)" (Utilities|Array|MakeArray ""))))))

(fn GetCraftingInformationbyEnum
  (params (EItem :type E_Item%20Enum :default "NewEnumerator1"))
  (bind _returnvalue (Utilities|GetDataTableRow "/Game/SurvivalKit/Blueprints/Datatables/DT_CraftingList.DT_CraftingList" (Utilities|String|StringToName (Utilities|String|EnumtoString EItem)))
    (:then
      (return _returnvalue))))

(fn GetSelectedSkinDetails
  (params (SkinList :type Array%20of%20S%20Item%20Skin%20Information%20Structures) (SkinName :type Name))
  (for _array_element SkinList
    (if (Utilities|Name|Equal(Name) (Utilities|Struct|BreakS_ItemSkinInformation _array_element) SkinName)
      (return _array_element true)))
  (return "" false))