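; Collectable world item actor for the survival kit, representing an inventory item placed in or dropped into the level.
; It looks up item data by type enum to set mesh transform, skin materials by slot name and physics.
; Initialization runs on construction, on BeginPlay for dropped items, and whenever new info arrives through a multicast setter.
; Dropped items simulating physics get a forward impulse; drag-and-drop and split-amount getters return zero.
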(event Custom|SetCollectableItemInfoMulticast
  (params (SCollectableItemInfo :type S%20Collectable%20Item%20Information%20Structure))
  ;[0.4277 0 1] Set Collectable Item Info
  (Variables|GeneralSettings|SetSCollectableItemInfo SCollectableItemInfo)
  (CollectableItem|InitializeCollectableItem))

(event EventSetCollectableItemInfo
  (params (SCollectableItemInfo :type S%20Collectable%20Item%20Information%20Structure))
  ;[0 1 0.4926] Set Item Information
  (CallFunction|SetCollectableItemInfoMulticast SCollectableItemInfo))

(event EventBeginPlay
  ;[0.09651 0 1] Event Construct
  (if (CollectableItem|IsItemDropped)
    (CollectableItem|InitializeCollectableItem)))

(fn ConstructionScript
  (CollectableItem|InitializeCollectableItem))

(fn IsItemDropped
  (return (Utilities|Struct|BreakS_CollectableItemInformation (Variables|GeneralSettings|GetSCollectableItemInfo))))

(fn InitializeCollectableItem
  (Variables|NonEditablePart|SetSItemInformation (CallFunction|GetItemInformationbyEnum (Utilities|Struct|BreakS_InventoryInformation (Utilities|Struct|BreakS_CollectableItemInformation (Variables|GeneralSettings|GetSCollectableItemInfo)))))
  (CollectableItem|InitializeItemSpawnSettings)
  (CollectableItem|InitializeItemVisualSettings)
  (CollectableItem|InitializeItemPhysicsSettings)
  (CollectableItem|InitializeItemImpulseSettings))

(fn InitializeItemSpawnSettings
  (bind _staticmesh (Variables|Default|GetStaticMesh))
  (bind _siteminformation (Variables|NonEditablePart|GetSItemInformation))
  (bind _sitemspawnsettings (Utilities|Struct|BreakS_ItemInformation _siteminformation))
  (bind (_sitemlocaloffset _sitemrotation _sitemscale) (Utilities|Struct|BreakS_ItemSpawnSettings _sitemspawnsettings))
  (Transformation|AddLocalOffset _staticmesh _sitemlocaloffset false false)
  (Transformation|SetWorldRotation _staticmesh _sitemrotation false false)
  (Transformation|SetWorldScale3D _staticmesh _sitemscale))

(fn InitializeItemVisualSettings
  (bind _siteminformation (Variables|NonEditablePart|GetSItemInformation))
  (bind (_sitemvisualsettings _sitemskinsettings) (Utilities|Struct|BreakS_ItemInformation _siteminformation))
  (Components|StaticMesh|SetStaticMesh (Variables|Default|GetStaticMesh) (Utilities|Struct|BreakS_ItemVisualSettings _sitemvisualsettings))
  (bind (_skininformation _issuccessful) (CallFunction|GetSelectedSkinDetails _sitemskinsettings (Utilities|Struct|BreakS_InventoryInformation (Utilities|Struct|BreakS_CollectableItemInformation (Variables|GeneralSettings|GetSCollectableItemInfo)))))
  (if _issuccessful
    (bind _keys (Utilities|Map|Keys (Utilities|Struct|BreakS_ItemSkinInformation _skininformation)))
    (bind _values (Utilities|Map|Values (Utilities|Struct|BreakS_ItemSkinInformation _skininformation)))
    (for (_array_element _array_index) _values
      (Rendering|Material|SetMaterialbyName (Variables|Default|GetStaticMesh) (Utilities|Array|Get(acopy) _keys _array_index) _array_element))))

(fn InitializeItemPhysicsSettings
  (bind _staticmesh (Variables|Default|GetStaticMesh))
  (bind _siteminformation (Variables|NonEditablePart|GetSItemInformation))
  (bind _sitemphysicssettings (Utilities|Struct|BreakS_ItemInformation _siteminformation))
  (bind (_issimulatingphysics _smassinkgsettings _lineardamping _angulardamping _enablegravity _ignoreradialimpulse _ingoreradialforce _applyimpulseondamage _replicatephyiscstoautonomousproxy) (Utilities|Struct|BreakS_ItemPhysicsSettings _sitemphysicssettings))
  (bind (_bonename _ismassinkgenabled _massinkg) (Utilities|Struct|BreakS_MassInKgSettings _smassinkgsettings))
  (Physics|SetSimulatePhysics _staticmesh (and (Utilities|Struct|BreakS_CollectableItemInformation (Variables|GeneralSettings|GetSCollectableItemInfo)) _issimulatingphysics))
  (Class|PrimitiveComponent|SetMassOverrideinKg _staticmesh _bonename _massinkg _ismassinkgenabled)
  (Class|PrimitiveComponent|SetLinearDamping _staticmesh _lineardamping)
  (Class|PrimitiveComponent|SetAngularDamping _staticmesh _angulardamping)
  (Physics|SetEnableGravity _staticmesh _enablegravity)
  (Variables|/Script/Engine.PrimitiveComponent|SetbIgnoreRadialImpulse _staticmesh _ignoreradialimpulse)
  (Variables|/Script/Engine.PrimitiveComponent|SetbIgnoreRadialForce _staticmesh _ingoreradialforce)
  (Variables|/Script/Engine.PrimitiveComponent|SetbApplyImpulseOnDamage _staticmesh _applyimpulseondamage)
  (Variables|/Script/Engine.PrimitiveComponent|SetbReplicatePhysicsToAutonomousProxy _staticmesh _replicatephyiscstoautonomousproxy))

(fn InitializeItemImpulseSettings
  (bind _siteminformation (Variables|NonEditablePart|GetSItemInformation))
  (bind _sitemimpulsesettings (Utilities|Struct|BreakS_ItemInformation _siteminformation))
  (bind (_impulsemultiplier _bonename _velchange) (Utilities|Struct|BreakS_ItemImpulseSettings _sitemimpulsesettings))
  (if (and (Utilities|Struct|BreakS_CollectableItemInformation (Variables|GeneralSettings|GetSCollectableItemInfo)) (Class|SceneComponent|IsAnySimulatingPhysics (Variables|Default|GetStaticMesh)))
    (Physics|AddImpulse (Variables|Default|GetStaticMesh) (* (Transformation|GetActorForwardVector) _impulsemultiplier) _bonename _velchange)))

(fn GetCollectableItemInfo
  (return (Variables|GeneralSettings|GetSCollectableItemInfo)))

(fn GetDragandDropInformation
  (return 0))

(fn GetSplittedItemAmount
  (return 0))