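; BP_ModularCharacter is a character built from separate skeletal meshes for head, hip, arms, legs and feet.
; The construction script makes each part follow the main Mesh through master pose, then caches that mesh and its skeletal child components alongside their default meshes in parallel arrays.
; Lookup functions use component tags to return a part's component or its original default mesh.
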(fn ConstructionScript
  (Class|SkinnedMeshComponent|SetMasterPoseComponent (Variables|Default|GetLeftFoot) (Variables|Character|GetMesh) false)
  (ModulerCharacter|InitializeModulerCharacter))

(fn InitializeModulerCharacter
  (bind _mesh (Variables|Character|GetMesh))
  (Utilities|Array|Add (Variables|NonEditablePart|GetDefaultSkeletalMeshes) (Variables|/Script/Engine.SkinnedMeshComponent|GetSkeletalMesh (Variables|Character|GetMesh)))
  (Utilities|Array|Add (Variables|ModulerCharacterSystem|GetSkeletalMeshComponents) _mesh)
  (for _array_element (Components|GetChildrenComponents _mesh false)
    (bind _asskeletal_mesh_component (Utilities|Casting|CastToSkeletalMeshComponent _array_element))
    (Utilities|Array|Add (Variables|ModulerCharacterSystem|GetSkeletalMeshComponents) _asskeletal_mesh_component)
    (Utilities|Array|Add (Variables|NonEditablePart|GetDefaultSkeletalMeshes) (Variables|/Script/Engine.SkinnedMeshComponent|GetSkeletalMesh _asskeletal_mesh_component))))

(fn GetSkeletalMeshComponentbyString
  (params (MeshComponentTagName :type Name))
  (for _array_element (Variables|ModulerCharacterSystem|GetSkeletalMeshComponents)
    (if (Utilities|Array|ContainsItem (Variables|/Script/Engine.ActorComponent|GetComponentTags _array_element) MeshComponentTagName)
      (return true _array_element)))
  (return false 0))

(fn GetDefaultSkeletalMeshesbyName
  (params (MeshComponentTagName :type Name))
  (for (_array_element _array_index) (Variables|ModulerCharacterSystem|GetSkeletalMeshComponents)
    (if (Utilities|Array|ContainsItem (Variables|/Script/Engine.ActorComponent|GetComponentTags _array_element) MeshComponentTagName)
      (return true (Utilities|Array|Get(acopy) (Variables|NonEditablePart|GetDefaultSkeletalMeshes) _array_index))))
  (return false 0))