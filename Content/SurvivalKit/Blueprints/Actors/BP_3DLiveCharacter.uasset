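; Live 3D preview double of the player character, filmed by a scene capture that hides the other actors present at initialization.
; Rebuilds the character's skeletal parts, socketed static clothing and materials via BPI_Character, refreshing them when SurvivalKitComponent reports clothing changes.
; Cursor deltas feed a clamped yaw target that Tick interpolates toward.
; With OptimizeWidgets enabled, capture starts disabled and is toggled through UpdateSceneCaptureStatus.
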(event Custom|EventBinding
  ;[0.5725 0 1] Event Binding
  (EventDispatchers|AssignOnCharacterClothesUpdated (Variables|Default|GetSurvivalKitComponent) (delegate Custom|OnCharacterClothesUpdated_Event_0)))

(event Custom|OnCharacterClothesUpdated_Event_0
  ;[0.5725 0 1] Event Binding
  (LiveCharacterSystem|UpdateLiveCharacter))

(event EventBeginPlay
  ;[0 0.2801 1] Begin Play
  (LiveCharacterSystem|InitializeLiveCharacter)
  (CallFunction|EventBinding))

(event EventUpdateCharacterRotation
  (params (CursorDelta :type Float%20%28double-precision%29))
  ;[0 0.7543 1] Update Character Rotation
  (LiveCharacterSystem|AddCursorDelta CursorDelta))

(event EventTick
  (params (DeltaSeconds :type Float%20%28single-precision%29))
  ;[0.2159 0 1] Event Tick
  (LiveCharacterSystem|RotateCharacterMesh))

(event EventUpdateSceneCaptureStatus
  (params (IsActive :type Boolean))
  ;[1 0 0] Update Scene Capture
  (LiveCharacterSystem|ToggleSceneCaptureStatus IsActive))

(fn ConstructionScript)

(fn RotateCharacterMesh
  (bind _scene (Variables|Default|GetScene))
  (if (LiveCharacterSystem|CharacterRotationConditions)
    (Transformation|SetRelativeRotation _scene (Math|Rotator|MakeRotator 0.0 0.0 (Math|Interpolation|FInterpTo (.yaw (Variables|/Script/Engine.SceneComponent|GetRelativeRotation _scene)) (.yaw (Variables|NonEditablePart|GetTotalCharacterRotation)) (Utilities|Time|GetWorldDeltaSeconds) (Variables|RotationSettings|GetRotationSpeedInterpSpeed))) false false)))

(fn AddCursorDelta
  (params (CursorDelta :type Float%20%28double-precision%29))
  (bind _saxisclamp (Variables|RotationSettings|GetSAxisClamp))
  (bind (_minimumclampvalue _maximumclampvalue) (Utilities|Struct|BreakS_XAxisClamp _saxisclamp))
  (Variables|NonEditablePart|SetTotalCharacterRotation (Math|Rotator|MakeRotator 0.0 0.0 (Math|Float|Clamp(Float) (+ (* CursorDelta (Variables|RotationSettings|GetRotationSpeedMultiplier) (select (Variables|RotationSettings|GetIsReverseAxis) 1.0 -1.0)) (.yaw (Variables|NonEditablePart|GetTotalCharacterRotation))) _minimumclampvalue _maximumclampvalue))))

(fn CharacterRotationConditions
  (return (Utilities|Enum|NotEqual(Enum) (Variables|NonEditablePart|GetTotalCharacterRotation) "0, 0, 0")))

(fn InitializeLiveCharacter
  (bind _returnvalue (CallFunction|GetSurvivalKitComponent (Variables|NonEditablePart|GetControllerReference)))
  (Variables|Default|SetSurvivalKitComponent _returnvalue)
  (LiveCharacterSystem|InitializeSkeletalMeshComponents)
  (LiveCharacterSystem|InitializeAttachedStaticMeshes)
  (LiveCharacterSystem|SetHiddenActors)
  (LiveCharacterSystem|ToggleSceneCaptureStatus false))

(fn UpdateLiveCharacter
  (if (Utilities|DoesObjectImplementInterface (Variables|/Game/SurvivalKit/Blueprints/Components/BP_SurvivalKitComponent.BP_SurvivalKitComponent_C|GetCharacterReference (Variables|Default|GetSurvivalKitComponent)) "/Game/SurvivalKit/Blueprints/Interfaces/BPI_Character.BPI_Character_C")
    (LiveCharacterSystem|UpdateSkeletalMeshComponents)
    (LiveCharacterSystem|UpdateAttachedStaticMeshes)))

(fn InitializeSkeletalMeshComponents
  (bind _survivalkitcomponent (Variables|Default|GetSurvivalKitComponent))
  (bind _characterreference (Variables|/Game/SurvivalKit/Blueprints/Components/BP_SurvivalKitComponent.BP_SurvivalKitComponent_C|GetCharacterReference _survivalkitcomponent))
  (if (Utilities|DoesObjectImplementInterface _characterreference "/Game/SurvivalKit/Blueprints/Interfaces/BPI_Character.BPI_Character_C")
    (bind _returnvalue (Class|BPICharacter|GetSkeletalMeshComponents(Message) _characterreference))
    (for _array_element _returnvalue
      (bind _returnvalue_2 (AddComponent|AddSkeletalMeshComponent false))
      (Components|SkinnedMesh|SetSkinnedAssetandUpdate _returnvalue_2 (Variables|/Script/Engine.SkinnedMeshComponent|GetSkeletalMesh _array_element) true)
      (LiveCharacterSystem|CopyMeshMaterial _array_element _returnvalue_2)
      (Transformation|AttachComponentToComponent _returnvalue_2 (Variables|Default|GetScene) "None" "SnapToTarget" "SnapToTarget" "SnapToTarget" true)
      (Utilities|Array|Add (Variables|NonEditablePart|GetSkeletalMeshParts) _returnvalue_2))))

(fn InitializeAttachedStaticMeshes
  (bind _returnvalue (Class|BPICharacter|GetAttachedClothStaticMeshComponents(Message) (Variables|/Game/SurvivalKit/Blueprints/Components/BP_SurvivalKitComponent.BP_SurvivalKitComponent_C|GetCharacterReference (Variables|Default|GetSurvivalKitComponent))))
  (for _array_element _returnvalue
    (bind _returnvalue_2 (AddComponent|AddStaticMeshComponent false))
    (Components|StaticMesh|SetStaticMesh _returnvalue_2 (Variables|/Script/Engine.StaticMeshComponent|GetStaticMesh _array_element))
    (LiveCharacterSystem|CopyMeshMaterial _array_element _returnvalue_2)
    (Transformation|AttachComponentToComponent _returnvalue_2 (Utilities|Array|Get(acopy) (Variables|NonEditablePart|GetSkeletalMeshParts)) (Transformation|GetAttachSocketName _array_element) "SnapToTarget" "SnapToTarget" "SnapToTarget" true)
    (Transformation|SetRelativeTransform _returnvalue_2 (Transformation|GetRelativeTransform _array_element) false false)
    (Utilities|Array|Add (Variables|NonEditablePart|GetAttachedStaticMeshComponentReferences) _returnvalue_2)))

(fn UpdateSkeletalMeshComponents
  (bind _returnvalue (Class|BPICharacter|GetSkeletalMeshComponents(Message) (Variables|/Game/SurvivalKit/Blueprints/Components/BP_SurvivalKitComponent.BP_SurvivalKitComponent_C|GetCharacterReference (Variables|Default|GetSurvivalKitComponent))))
  (for (_array_element _array_index) _returnvalue
    (Components|SkinnedMesh|SetSkinnedAssetandUpdate (Utilities|Array|Get(acopy) (Variables|NonEditablePart|GetSkeletalMeshParts) _array_index) (Variables|/Script/Engine.SkinnedMeshComponent|GetSkeletalMesh _array_element) false)
    (LiveCharacterSystem|CopyMeshMaterial _array_element (Utilities|Array|Get(acopy) (Variables|NonEditablePart|GetSkeletalMeshParts) _array_index))))

(fn UpdateAttachedStaticMeshes
  (LiveCharacterSystem|ClearAttachedStaticMeshes)
  (LiveCharacterSystem|InitializeAttachedStaticMeshes))

(fn ClearAttachedStaticMeshes
  (for _array_element (Variables|NonEditablePart|GetAttachedStaticMeshComponentReferences)
    (Components|DestroyComponent _array_element))
  (Utilities|Array|Clear (Variables|NonEditablePart|GetAttachedStaticMeshComponentReferences)))

(fn CopyMeshMaterial
  (params (MeshComponentToBeCopied :type Mesh%20Component%20Object%20Reference) (TargetPrimitiveComponent :type Primitive%20Component%20Object%20Reference))
  (for (_array_element _array_index) (Rendering|Material|GetMaterials MeshComponentToBeCopied)
    (Rendering|Material|SetMaterial TargetPrimitiveComponent _array_index _array_element)))

(fn SetHiddenActors
  (bind _outactors (Actor|GetAllActorsOfClass "/Script/Engine.Actor"))
  (Utilities|Array|RemoveItem _outactors self)
  (Variables|/Script/Engine.SceneCaptureComponent|SetHiddenActors (Variables|Default|GetSceneCaptureComponent2D) _outactors))

(fn ToggleSceneCaptureStatus
  (params (IsActive :type Boolean))
  (bind _scenecapturecomponent2d (Variables|Default|GetSceneCaptureComponent2D))
  (if (Variables|/Game/SurvivalKit/Blueprints/Components/BP_SurvivalKitComponent.BP_SurvivalKitComponent_C|GetOptimizeWidgets (Variables|Default|GetSurvivalKitComponent))
    (bind _output_get (Variables|/Script/Engine.SceneCaptureComponent|SetbCaptureEveryFrame _scenecapturecomponent2d IsActive))
    (Variables|/Script/Engine.SceneCaptureComponent|SetbCaptureOnMovement _scenecapturecomponent2d _output_get)))

(fn GetCharacterReference
  (return (Variables|/Game/SurvivalKit/Blueprints/Components/BP_SurvivalKitComponent.BP_SurvivalKitComponent_C|GetCharacterReference (Variables|Default|GetSurvivalKitComponent))))