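; Survival Kit game instance that owns the save game object for the game session.
; On Init it loads the named slot if it exists, otherwise creates a new save object of the target class without writing it to disk.
; Getters expose the save reference and slot name.
; IsSaveGameInventoryInitilaized returns true when the saved inventory is empty, the opposite of what its name suggests.
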(event EventInit
  ;[0.04151 1 0] Event Init
  (CallFunction|InitializeSaveGame))

(fn InitializeSaveGame
  (bind _returnvalue (SaveGame|DoesSaveGameExist (Variables|ConfigurableSettings|GetSaveGameName)))
  (if _returnvalue
    (bind _returnvalue_2 (SaveGame|LoadGamefromSlot (Variables|ConfigurableSettings|GetSaveGameName)))
    (Variables|NonEditablePart|SetSaveGameReference _returnvalue_2)
    (else
      (bind _returnvalue_3 (SaveGame|CreateSaveGameObject (LocalVariables|GetTargetSaveGameClass)))
      (Variables|NonEditablePart|SetSaveGameReference _returnvalue_3))))

(fn GetSaveGameReference
  (return (Variables|NonEditablePart|GetSaveGameReference)))

(fn GetSaveGameSlotName
  (return (Variables|ConfigurableSettings|GetSaveGameName)))

(fn IsSaveGameInventoryInitilaized
  (bind _ssavegameinformations (Class|BPISaveGame|GetSaveGameInformations(Message) (Variables|NonEditablePart|GetSaveGameReference)))
  (return (<= (Utilities|Array|Length (.MyInventory (Utilities|Struct|BreakS_SaveGameInventoryInfo _ssavegameinformations))) 0)))