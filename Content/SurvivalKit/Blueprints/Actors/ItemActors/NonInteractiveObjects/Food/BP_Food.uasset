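; BP_Food is the item actor for edible food in the survival kit, consumed through quick use or the eat action.
; Both events call EatItemFood, which sends the food struct to the character, removes one unit from the inventory slot, plays the use sound and destroys the item.
; GetItemInformation exposes the instant health, hunger and thirst values as a labeled map.
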(event EventBeginPlay
  (|CallParentFunction) ; This node is disabled and will not be called.\nDrag off pins to build functionality.
)

(event Collision|EventActorBeginOverlap
  (params (OtherActor :type Actor%20Object%20Reference))
  (|CallParentFunction OtherActor) ; This node is disabled and will not be called.\nDrag off pins to build functionality.
)

(event EventTick
  (params (DeltaSeconds :type Float%20%28single-precision%29))
  (|CallParentFunction DeltaSeconds) ; This node is disabled and will not be called.\nDrag off pins to build functionality.
)

(event EventQuickUseItem
  ;[1 0 0.02832] Event Use Item
  (GeneralFunctions|EatItemFood))

(event EventActionEatItem
  ;[1 0.532 0] Use Action Interface Function
  (GeneralFunctions|EatItemFood))

(fn ConstructionScript
  (|CallParentFunction))

(fn GetItemInformation
  (bind _sfoodinformation (Variables|FoodCategory|GetSFoodInformation))
  (bind (_instanthealth _hunger _thirst) (Utilities|Struct|BreakS_FoodItemInformation _sfoodinformation))
  (return (Utilities|Map|MakeMap "Instant Health" _instanthealth "Hunger" _hunger "Thirst" _thirst)))

(fn EatItemFood
  (Class|BPICharacter|EatFood(Message) (Variables|/Game/SurvivalKit/Blueprints/Components/BP_SurvivalKitComponent.BP_SurvivalKitComponent_C|GetCharacterReference (Variables|Default|GetSurvivalKitComponent)) (Variables|FoodCategory|GetSFoodInformation))
  (Default|DeleteSlotfromInventory (Variables|Default|GetSurvivalKitComponent) (Utilities|Struct|MakeS_InventorySlotDeleteInformation (Variables|Default|GetSlotID) 1) true)
  (CallFunction|PlayItemUsedSoundClient)
  (CallFunction|DestroyItemMulticast))