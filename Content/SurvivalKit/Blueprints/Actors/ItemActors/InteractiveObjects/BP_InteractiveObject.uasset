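; BP_InteractiveObject is a base item actor for usable physical objects in the survival kit, with a use event meant for override in derived classes.
; Quick use snaps it to a socket on the owning character's master pose mesh, or destroys it via multicast if the socket is missing.
; BeginPlay and Destroyed notify the SurvivalKitComponent to toggle the mainbar slot's selected state.
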(event Custom|ToggleObjectAttachStatus
  ;[0.1686 0 1] Event Quick Use Item
  (bind _survivalkitcomponent (Variables|Default|GetSurvivalKitComponent)
    (:then
      (bind _returnvalue (Class|BPICharacter|GetMasterPoseComponent(Message) (Variables|/Game/SurvivalKit/Blueprints/Components/BP_SurvivalKitComponent.BP_SurvivalKitComponent_C|GetCharacterReference _survivalkitcomponent)))
      (if (Transformation|DoesSocketExist _returnvalue (Variables|PhysicalObjectSettings|GetSocketName))
        (Transformation|AttachComponentToComponent self _returnvalue (Variables|PhysicalObjectSettings|GetSocketName) "SnapToTarget" "SnapToTarget" "SnapToTarget" true)
        (else
          (CallFunction|DestroyItemMulticast))))
    (:else)))

(event EventBeginPlay
  ;[0 0.7012 1] Begin Play
  (|CallParentFunction)
  (bind _survivalkitcomponent (Variables|Default|GetSurvivalKitComponent)
    (:then
      (Default|CallOnMainbarSlotToggled _survivalkitcomponent (Variables|Default|GetSlotID) true))
    (:else)))

(event EventQuickUseItem
  ;[0 0.2803 1] Quick Use Item
  (CallFunction|ToggleObjectAttachStatus))

(event EventUsePhysicalItem
  ;[1 0 0] Use Physical Item Event
  (Development|PrintString "Please Override Use Physical Item Event, In Derived Class."))

(event EventDestroyed
  ;[0 1 0.7172] Event Destroyed
  (bind _survivalkitcomponent (Variables|Default|GetSurvivalKitComponent)
    (:then
      (Default|CallOnMainbarSlotToggled _survivalkitcomponent (Variables|Default|GetSlotID) false))
    (:else)))

(fn ConstructionScript
  (|CallParentFunction))

(fn GetItemInformation
  (return (|CallParentFunction)))

(fn GetUsePhysicalItemKey
  (return (Variables|PhysicalObjectSettings|GetUsePhysicalItemKey)))