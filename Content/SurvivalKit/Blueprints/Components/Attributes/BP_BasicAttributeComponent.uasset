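; Survival-kit attribute component that holds a character stat, optionally clamped and changed by random amounts at random timer intervals.
; Value changes fire a change event, also raised on RepNotify, whose bound handling saves to the save game slot; BeginPlay restores it by class.
; While below a configured threshold, it can run a second timer that modifies another attribute component on the character, letting one stat affect another.
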(event Custom|StartChangeValueOverTime
  ;[0.3328 0 1] Start Change Value Over Time
  (Utilities|Time|SetTimerbyEvent (delegate Custom|ChangeValue) (GetterFunctions|GetRandomChangingValueTime)))

(event Custom|ChangeValue
  ;[0.3328 0 1] Start Change Value Over Time
  (CallFunction|UpdateCurrentValue (GetterFunctions|GetRandomChangingValue))
  (CallFunction|StartChangeValueOverTime))

(event Custom|ModifyAttributeValue
  (params (AddCurrentValueTo :type Float%20%28double-precision%29))
  ;[1 0.07806 0] Modify Attribute Value
  (SetterFunction|SetAttributeValue (+ (GetterFunctions|GetCurrentValue) AddCurrentValueTo)))

(event Custom|OnReachedMaximumValue
  ;[0 1 0.6817] On Reached Maximum Value
)

(event Custom|StartChangingTargetCompTimer
  ;[0.9061 0 1] Start Changing Target Value
  (bind _returnvalue (Utilities|Time|SetTimerbyEvent (delegate Custom|ChangeTargetComponent) (GetterFunctions|GetTargetComponentChangingValueTime)))
  (Variables|NonEditablePart|SetTargetComponentTimer _returnvalue))

(event Custom|ChangeTargetComponent
  ;[0.9061 0 1] Start Changing Target Value
  (if (GetterFunctions|IsCurrentValueBelowCertainLevel)
    (CallFunction|UpdateCurrentValue (Variables|Default|GetTargetAttributeReference) (GetterFunctions|GetTargetComponentChangeValue))
    (CallFunction|StartChangingTargetCompTimer)))

(event Custom|OnReachedMinmumValue
  ;[0.2941 0 1] On Reached Minimum Value
)

(event EventBeginPlay
  ;[1 0.02049 0] Begin Play
  (|CallParentFunction)
  (|EventBinding)
  (BasicAttribute|InitializeBasicAttribute))

(event EventUpdateCurrentValue
  (params (ValueToAdd :type Float%20%28double-precision%29))
  ;[0 1 0.2716] Update Current Value
  (CallFunction|ModifyAttributeValue ValueToAdd))

(fn InitializeBasicAttribute
  (if (GetterFunctions|IsChangingOverTime)
    (CallFunction|StartChangeValueOverTime))
  (BasicAttribute|LoadAttributeValue)
  (bind _returnvalue (Class|BPICharacter|GetTargetAttributeReference(Message) (Variables|Default|GetCharacterReference) (GetterFunctions|GetTargetComponentClass)))
  (Variables|Default|SetTargetAttributeReference _returnvalue))

(fn IsChangingOverTime
  (return (.IsChangingOverTime (Utilities|Struct|BreakS_BasicAttributeChangeInformation (Utilities|Struct|BreakS_BasicAttributeInformation (Variables|BasicAttribute|GetBasicAttributeInformation))))))

(fn GetRandomChangingValueTime
  (bind _basicattributeinformation (Variables|BasicAttribute|GetBasicAttributeInformation))
  (bind _attributechangeinformation (Utilities|Struct|BreakS_BasicAttributeInformation _basicattributeinformation))
  (bind (_minmumchangevalue _maximumchangevalue _minimumdecreasevaluetime _maximumdecreasevaluetime) (Utilities|Struct|BreakS_BasicAttributeChangeInformation _attributechangeinformation))
  (return (Math|Random|RandomFloatinRange _minimumdecreasevaluetime _maximumdecreasevaluetime)))

(fn GetCurrentValue
  (return (Utilities|Struct|BreakS_BasicAttributeGeneralInformation (Utilities|Struct|BreakS_BasicAttributeInformation (Variables|BasicAttribute|GetBasicAttributeInformation)))))

(fn GetRandomChangingValue
  (bind _basicattributeinformation (Variables|BasicAttribute|GetBasicAttributeInformation))
  (bind _attributechangeinformation (Utilities|Struct|BreakS_BasicAttributeInformation _basicattributeinformation))
  (bind (_minmumchangevalue _maximumchangevalue) (Utilities|Struct|BreakS_BasicAttributeChangeInformation _attributechangeinformation))
  (return (Math|Random|RandomFloatinRange _minmumchangevalue _maximumchangevalue)))

(fn OnAttributeValueUpdated
  (GetterFunctions|CheckIsValueBelowValue)
  (BasicAttribute|SaveAttributeValue))

(fn GetTargetComponentClass
  (return (.TargetComponent (Utilities|Struct|BreakS_BasicAttibuteOthers (Utilities|Struct|BreakS_BasicAttributeInformation (Variables|BasicAttribute|GetBasicAttributeInformation))))))

(fn GetTargetComponentChangeValue
  (bind _basicattributeinformation (Variables|BasicAttribute|GetBasicAttributeInformation))
  (bind _attributeothers (Utilities|Struct|BreakS_BasicAttributeInformation _basicattributeinformation))
  (bind (_minimumchangevalue _maximumchangevalue) (Utilities|Struct|BreakS_BasicAttibuteOthers _attributeothers))
  (return (Math|Random|RandomFloatinRange _minimumchangevalue _maximumchangevalue)))

(fn GetTargetComponentChangingValueTime
  (bind _basicattributeinformation (Variables|BasicAttribute|GetBasicAttributeInformation))
  (bind _attributeothers (Utilities|Struct|BreakS_BasicAttributeInformation _basicattributeinformation))
  (bind (_minimumchangevalueticktime _maximumchangevalueticktime) (Utilities|Struct|BreakS_BasicAttibuteOthers _attributeothers))
  (return (Math|Random|RandomFloatinRange _minimumchangevalueticktime _maximumchangevalueticktime)))

(fn IsCurrentValueBelowCertainLevel
  (return (< (GetterFunctions|GetCurrentValue) (Utilities|Struct|BreakS_BasicAttibuteOthers (Utilities|Struct|BreakS_BasicAttributeInformation (Variables|BasicAttribute|GetBasicAttributeInformation))))))

(fn CheckIsValueBelowValue
  (bind _targetcomponenttimer (Variables|NonEditablePart|GetTargetComponentTimer))
  (bind _returnvalue (Utilities|Time|IsTimerActivebyHandle _targetcomponenttimer))
  (if (GetterFunctions|IsTargetComponentChangingActive)
    (if (GetterFunctions|IsCurrentValueBelowCertainLevel)
      (if (not _returnvalue)
        (CallFunction|StartChangingTargetCompTimer))
      (elif _returnvalue
        (Utilities|Time|ClearandInvalidateTimerbyHandle (Variables|NonEditablePart|GetTargetComponentTimer))))))

(fn IsTargetComponentChangingActive
  (return (Utilities|Struct|BreakS_BasicAttibuteOthers (Utilities|Struct|BreakS_BasicAttributeInformation (Variables|BasicAttribute|GetBasicAttributeInformation)))))

(fn LoadAttributeValue
  (bind _returnvalue (Class|BPIGameInstance|GetSaveGameReference(Message) (Game|GetGameInstance)))
  (bind (_returnvalue_2 _isregistered) (Class|BPISaveGame|GetBasicAttributeValue(Message) _returnvalue (Utilities|GetClass self)))
  (if _isregistered
    (SetterFunction|SetAttributeValue _returnvalue_2)))

(fn SetAttributeValue
  (params (CurrentValue :type Float%20%28double-precision%29))
  (bind _structout (Utilities|Struct|SetmembersinS_BasicAttributeGeneralInformation (Utilities|Struct|BreakS_BasicAttributeInformation (Variables|BasicAttribute|GetBasicAttributeInformation)) (BasicAttribute|CheckModifyingValue CurrentValue)))
  (Utilities|Struct|SetmembersinS_BasicAttributeInformation (Variables|BasicAttribute|GetBasicAttributeInformation) _structout)
  (Default|CallOnAttributeValueChanged))

(fn SaveAttributeValue
  (bind _returnvalue (Game|GetGameInstance))
  (bind _returnvalue_2 (Class|BPIGameInstance|GetSaveGameReference(Message) _returnvalue))
  (bind _returnvalue_3 (Class|BPIGameInstance|GetSaveGameSlotName(Message) _returnvalue))
  (Class|BPISaveGame|SetBasicAttributeValue(Message) _returnvalue_2 (Utilities|GetClass self) (GetterFunctions|GetCurrentValue))
  (SaveGame|SaveGametoSlot _returnvalue_2 _returnvalue_3))

(fn CheckModifyingValue
  (params (ValueToChangeAttribute :type Float%20%28double-precision%29))
  (bind _basicattributeinformation (Variables|BasicAttribute|GetBasicAttributeInformation))
  (bind _attributegeneralinformation (Utilities|Struct|BreakS_BasicAttributeInformation _basicattributeinformation))
  (bind (_minmumvalue _maximumvalue) (Utilities|Struct|BreakS_BasicAttributeGeneralInformation _attributegeneralinformation))
  (return (select (Variables|ConfigurableSettings|GetActivateValueClamping) (Math|Float|Clamp(Float) ValueToChangeAttribute _minmumvalue _maximumvalue) ValueToChangeAttribute)))

(fn OnRepBasicAttributeInformation
  (Default|CallOnAttributeValueChanged))

(fn GetAttributeInformation
  (return 0.0 0.0 0.0))

(fn GetAttributeVisualSettings
  (return 0 ""))