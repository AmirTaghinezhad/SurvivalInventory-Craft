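; BP_Medical is an item actor for medicine that a character uses from the inventory in the survival kit.
; Quick use and the use-medicines action share one path: it sends the medical data to the character through an interface message, removes one unit from the inventory slot, plays a sound and destroys the item.
; GetItemInformation exposes the instant health value as a labelled map entry.
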(event EventActionUseMedicines
  ;[0.01338 0 1] Use Medinice Interface Function
  (Class|BPICharacter|TakeMedicine(Message) (Variables|/Game/SurvivalKit/Blueprints/Components/BP_SurvivalKitComponent.BP_SurvivalKitComponent_C|GetCharacterReference (Variables|Default|GetSurvivalKitComponent)) (Variables|InventorySystem|GetSMedicalInformation))
  (Default|DeleteSlotfromInventory (Variables|Default|GetSurvivalKitComponent) (Utilities|Struct|MakeS_InventorySlotDeleteInformation (Variables|Default|GetSlotID) 1) false)
  (CallFunction|PlayItemUsedSound)
  (CallFunction|DestroyItem))

(event EventQuickUseItem
  ;[1 0 0.02338] Overriden Quick Use Item
  ;[0.01338 0 1] Use Medinice Interface Function
  (Class|BPICharacter|TakeMedicine(Message) (Variables|/Game/SurvivalKit/Blueprints/Components/BP_SurvivalKitComponent.BP_SurvivalKitComponent_C|GetCharacterReference (Variables|Default|GetSurvivalKitComponent)) (Variables|InventorySystem|GetSMedicalInformation))
  (Default|DeleteSlotfromInventory (Variables|Default|GetSurvivalKitComponent) (Utilities|Struct|MakeS_InventorySlotDeleteInformation (Variables|Default|GetSlotID) 1) false)
  (CallFunction|PlayItemUsedSound)
  (CallFunction|DestroyItem))

(fn ConstructionScript
  (|CallParentFunction))

(fn GetItemInformation
  (return (Utilities|Map|MakeMap "Instant Health" (Utilities|Struct|BreakS_MedicalItemInformation (Variables|InventorySystem|GetSMedicalInformation)))))