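; BP_Clothes is a non-interactive item actor that represents a piece of clothing in the survival kit.
; It exposes the fields of its cloth information struct as a name-keyed map of resistance stats covering combat, temperature and bleed-style protection.
; Getters also return its cloth type and the types it is incompatible with.
; It is a data holder, with no active event logic of its own.
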(event EventBeginPlay
  (|CallParentFunction) ; This node is disabled and will not be called.\nDrag off pins to build functionality.
)

(fn ConstructionScript
  (|CallParentFunction))

(fn GetItemInformation
  (bind _sclothiteminformation (Variables|ClothSystem|GetSClothItemInformation))
  (bind (_meleeresistance _weaponresistance _coldresistance _heatresistance _rangeresitance _bloodyresistance) (Utilities|Struct|BreakS_ClothItemInformation _sclothiteminformation))
  (return (Utilities|Map|MakeMap "Melee Resistance" _meleeresistance "Weapon Resistance" _weaponresistance "Cold Resistance" _coldresistance "Heat Resistance" _heatresistance "Range Reistance" _rangeresitance "Bloody Resistance" _bloodyresistance)))

(fn GetClothType
  (return (Variables|ClothSystem|GetEClothType)))

(fn GetinCompatibleClothTypes
  (return (Variables|ClothSystem|GetEInCompatibleTypes)))